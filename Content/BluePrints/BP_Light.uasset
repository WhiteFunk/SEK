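; BP_Light is a light actor whose PointLight flickers on and off a set number of times after play starts.
; Tick runs through a one-second Delay into a DoN gate capped at twice NumberOfFlickers, calling TurnOnOff to invert the light's visibility on each pass.
; The construction script repeats that toggle logic inline, so each construction run also inverts the light's visibility.
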(event `self.ReceiveBeginPlay`)

(event `self.ReceiveTick`
  (params (DeltaSeconds :type "Float (single-precision)"))
  (`KismetSystemLibrary.Delay` 1.0)
  (`/Engine/EditorBlueprintResources/StandardMacros.Do N` (* (`self.NumberOfFlickers`) 2)
    (:`Exit`
      (`self.TurnOn/Off`))))

(fn `TurnOn/Off`
  (if (`SceneComponent.IsVisible` (`self.PointLight`))
    (`SceneComponent.SetVisibility` (`self.PointLight`) false false)
    (else
      (`SceneComponent.SetVisibility` (`self.PointLight`) true false))))

(fn `UserConstructionScript`
  (if (`SceneComponent.IsVisible` (`self.PointLight`))
    (`SceneComponent.SetVisibility` (`self.PointLight`) false false)
    (else
      (`SceneComponent.SetVisibility` (`self.PointLight`) true false))))