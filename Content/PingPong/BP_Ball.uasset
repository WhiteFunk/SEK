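; BP_Ball is the ball actor for the PingPong game, moving in a straight line and bouncing off whatever it hits.
; Each Tick sweeps its Sphere along the normalized Direction by BSpeed, without delta-time scaling, so movement depends on frame rate.
; The sweep's impact normal then reflects Direction every frame, with no explicit hit check.
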(event `self.ReceiveBeginPlay`)

(event `self.ReceiveTick`
  (params (DeltaSeconds :type "Float (single-precision)"))
  (bind _sweephitresult (`SceneComponent.K2_AddWorldOffset` (`self.Sphere`) (* (`KismetMathLibrary.Normal` (`self.Direction`)) (`self.B_Speed`)) true false))
  (set `self.Direction` (`KismetMathLibrary.GetReflectionVector` (`self.Direction`) (`.ImpactNormal` (`GameplayStatics.BreakHitResult` _sweephitresult)))))

(fn `UserConstructionScript`)