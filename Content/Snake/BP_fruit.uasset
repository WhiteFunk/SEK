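; BP_fruit is the collectible fruit in a Snake game.
; Its Overlaped event, given the player, increments the score and adds a tail segment.
; It then asks the SnakeGM game mode to spawn the next fruit and destroys itself.
; Its own BeginPlay, overlap and Tick events are disabled, so the Overlaped event is triggered from outside this Blueprint.
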(event `self.Overlaped`
  (params (Player :type "/Game/Snake/BP_SnakePawn Object Reference"))
  (`/Game/Snake/BP_SnakePawn.IncrementScore` Player)
  (`/Game/Snake/BP_SnakePawn.AddTail` Player)
  (bind _assnake_gm (cast `/Game/Snake/SnakeGM` (`GameplayStatics.GetGameMode`)))
  (`/Game/Snake/SnakeGM.SpawnFruit` _assnake_gm)
  (`self.K2_DestroyActor`))

(fn `UserConstructionScript`
  (`parent.UserConstructionScript`))