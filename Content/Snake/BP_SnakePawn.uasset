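; BP_SnakePawn is the player-controlled snake, moving one head-mesh width every Tick along its current direction.
; Input events change direction only when the last move was not on that axis, preventing reversals.
; Each Tick shifts every tail actor into its predecessor's previous location.
; AddTail spawns a scaled-down BP_Tail using the head's mesh, while score events update the UI_Snake widget created on BeginPlay.
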(event `InputAction|Snake_Up`
  (params (Key :type "Key Structure"))
  (bind _currentmovedirection_x (`KismetMathLibrary.BreakVector` (`self.CurrentMoveDirection`)))
  ;[1 1 1] Input
  (:`Pressed`
    (if (== _currentmovedirection_x 0.0)
      (set `self.Direction` (1.0 0.0 0.0)))))

(event `InputAction|Snake_Down`
  (params (Key :type "Key Structure"))
  (bind _currentmovedirection_x (`KismetMathLibrary.BreakVector` (`self.CurrentMoveDirection`)))
  ;[1 1 1] Input
  (:`Pressed`
    (if (== _currentmovedirection_x 0.0)
      (set `self.Direction` (-1.0 0.0 0.0)))))

(event `InputAction|Snake_Right`
  (params (Key :type "Key Structure"))
  (bind (_currentmovedirection_x _currentmovedirection_y) (`KismetMathLibrary.BreakVector` (`self.CurrentMoveDirection`)))
  ;[1 1 1] Input
  (:`Pressed`
    (if (== _currentmovedirection_y 0.0)
      (set `self.Direction` (0.0 1.0 0.0)))))

(event `InputAction|Snake_Left`
  (params (Key :type "Key Structure"))
  (bind (_currentmovedirection_x _currentmovedirection_y) (`KismetMathLibrary.BreakVector` (`self.CurrentMoveDirection`)))
  ;[1 1 1] Input
  (:`Pressed`
    (if (== _currentmovedirection_y 0.0)
      (set `self.Direction` (0.0 -1.0 0.0)))))

(event `self.ReceiveBeginPlay`
  (bind _returnvalue (`StaticMesh.GetBoundingBox` (`StaticMeshComponent.StaticMesh` (`self.Head`))))
  (set `self.Step` (- (.x (`.Max` (break `Box` _returnvalue))) (.x (break `Box` _returnvalue))))
  (bind _returnvalue_2 (`|GenericCreateObject` "/Game/Snake/UI_Snake.UI_Snake_C"))
  (bind _output_get (set `self.UI` _returnvalue_2))
  (`UserWidget.AddToViewport` _output_get 0))

(event `self.ReceiveTick`
  (params (DeltaSeconds :type "Float (single-precision)"))
  (set `self.PreviousLocation` (`self.K2_GetActorLocation`))
  (`self.K2_AddActorWorldOffset` (* (`self.Direction`) (`self.Step`)))
  (set `self.CurrentMoveDirection` (- (`self.K2_GetActorLocation`) (`self.PreviousLocation`)))
  (for _array_element (`self.Tails`)
    (bind _output_get (set `self.TailCurrLocation` (`self.K2_GetActorLocation` _array_element)))
    (`self.K2_SetActorLocation` _array_element (`self.PreviousLocation`) false false)
    (set `self.PreviousLocation` _output_get)))

(event `DecrementScore`
  ;[1 1 1] Score
  (bind _result (`/Engine/EditorBlueprintResources/StandardMacros.DecrementInt` (`self.Score`))
    (:`  `
      (bind _output_get (set `self.Score` _result))
      (`/Game/Snake/UI_Snake.IncrementScore` (`self.UI`) _output_get))))

(event `IncrementScore`
  ;[1 1 1] Score
  (bind _result (`/Engine/EditorBlueprintResources/StandardMacros.IncrementInt` (`self.Score`))
    (:`  `
      (bind _output_get (set `self.Score` _result))
      (`/Game/Snake/UI_Snake.IncrementScore` (`self.UI`) _output_get))))

(event `AddTail`
  ;[1 1 1] Tail
  (bind _returnvalue (`|SpawnActorFromClass` "/Game/Snake/BP_Tail.BP_Tail_C" (`KismetMathLibrary.MakeTransform` (- (`self.K2_GetActorLocation`) (* (`self.Direction`) (`self.Step`))) (struct) (0.7 0.7 0.7)) "Undefined" "OverrideRootScale" null null))
  (`StaticMeshComponent.SetStaticMesh` (`/Game/Snake/BP_Abstract_Trigger.Mesh` _returnvalue) (`StaticMeshComponent.StaticMesh` (`self.Head`)))
  (`KismetArrayLibrary.Array_Add` (`self.Tails`) _returnvalue))

(fn `UserConstructionScript`)